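; BP_GrabMaster is a grabbable item actor, apparently a base class, configured by a mesh and a grab type.
; Its construction script applies the mesh to the Item component, then sets physics by grab type: one type simulates physics as PhysicsBody, any other is non-simulated WorldDynamic.
; GetGrabType exposes the type to callers; the event graph holds no active logic, so grab handling is not implemented here.
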(event EventBeginPlay)

(event Collision|EventActorBeginOverlap
  (params (OtherActor :type Actor%20Object%20Reference)))

(event EventTick
  (params (DeltaSeconds :type Float%20%28single-precision%29)))

(fn ConstructionScript
  (Components|StaticMesh|SetStaticMesh (Variables|Default|GetItem) (Variables|Default|Getmesh))
  (if (Utilities|Enum|Equal(Enum) (Variables|Default|GetGrab%20Type) "NewEnumerator1")
    (Physics|SetSimulatePhysics (Variables|Default|GetItem) true)
    (Collision|SetCollisionObjectType (Variables|Default|GetItem) "ECC_PhysicsBody")
    (else
      (Physics|SetSimulatePhysics (Variables|Default|GetItem) false)
      (Collision|SetCollisionObjectType (Variables|Default|GetItem) "ECC_WorldDynamic"))))

(fn GetGrabType
  (return (Variables|Default|GetGrab%20Type)))