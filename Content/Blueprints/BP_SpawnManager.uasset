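; BP_SpawnManager spawns BP_GravityEnemy actors over time until a cap is reached.
; A looping one-second timer started on BeginPlay compares CurrentEnemies to MaxEnemies, spawning and incrementing the count while at or below the limit.
; Each enemy appears at a random X and Y within a fixed bounding box, at a constant height.
; Nothing in this Blueprint decrements the count.
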(event Custom|Spawn
  (bind _returnvalue (Math|Random|RandomPointinBoundingBox "1020.000000,50.000000,350.000000" "1000.000000,2000.000000,0.000000"))
  (Game|SpawnActorfromClass "/Game/FirstPerson/Blueprints/Enemies/BP_GravityEnemy.BP_GravityEnemy_C" (Math|Transform|MakeTransform (Math|Vector|MakeVector (.x _returnvalue) (.y _returnvalue) 4.5e+02) "0, 0, 0" "1.000000,1.000000,1.000000") "Undefined" "MultiplyWithRoot" 0 0))

(event Custom|spawnTimer
  (if (<= (Variables|Default|GetcurrentEnemies) (Variables|Default|GetmaxEnemies))
    (CallFunction|Spawn)
    (Math|Integer|IncrementInt (Variables|Default|GetcurrentEnemies))))

(event EventBeginPlay
  (Utilities|Time|SetTimerbyEvent (delegate Custom|spawnTimer) 1.0 true)
  (if (<= (Variables|Default|GetcurrentEnemies) (Variables|Default|GetmaxEnemies))
    (CallFunction|Spawn)
    (Math|Integer|IncrementInt (Variables|Default|GetcurrentEnemies))))

(fn ConstructionScript)